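; BP_EnemyCharacter is an enemy character that shows its health and shield on an overhead WBP_HealthBar widget.
; On BeginPlay and on health or shield change events, it reads Ability System Component attributes and pushes current and max values to the widget.
; On damage, it prints the amount and causer, then spawns a BP_DamageInd carrying the damage, offset up and right from the health bar's head socket location.
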(event `self.ReceiveBeginPlay`
  (`self.UpdateHealth`)
  (`self.UpdateShield`))

(event `self.OnHealthChanged`
  (params (OldValue :type "Float (single-precision)") (NewValue :type "Float (single-precision)"))
  ; Health
  (`self.UpdateHealth`))

(event `self.OnShieldChanged`
  (params (OldValue :type "Float (single-precision)") (NewValue :type "Float (single-precision)"))
  (`self.UpdateShield`))

(event `self.OnDamageTaken`
  (params (DamageInstigator :type "Actor Object Reference") (DamageCauser :type "Actor Object Reference") (GameplayTagContainer :type "GameplayTagContainer Structure (by ref)") (Damage :type "Float (single-precision)"))
  ; Damage Taken
  (`KismetSystemLibrary.PrintString` (`KismetStringLibrary.Concat_StrStr` (`KismetStringLibrary.Conv_DoubleToString` Damage) " Damage from: " (`KismetSystemLibrary.GetDisplayName` DamageCauser)))
  (bind (_upvector _rightvector) (`self.IF_GetVectors` self))
  (`|SpawnActorFromClass` "/Game/Blueprint/BP_DamageInd.BP_DamageInd_C" (`KismetMathLibrary.MakeTransform` (+ (* _upvector 20.0) (* _rightvector 20.0) (`SceneComponent.GetSocketLocation` (`self.HealthBar`) "head"))) "Undefined" "MultiplyWithRoot" null Damage null))

(fn `IF_GetVectors`
  (returns (UpVector :type "Vector Structure") (RightVector :type "Vector Structure"))
  (bind _returnvalue (`self.K2_GetActorRotation`))
  (return (`KismetMathLibrary.GetUpVector` _returnvalue) (`KismetMathLibrary.GetRightVector` _returnvalue)))

(fn `UpdateHealth`
  (bind _abilitysystemcomponent (`self.AbilitySystemComponent`))
  (bind _aswbp_health_bar (cast `/Game/UI/WBP_HealthBar` (`WidgetComponent.GetUserWidgetObject` (`self.HealthBar`))))
  (`/Game/UI/WBP_HealthBar.UpdateHealth` _aswbp_health_bar (`.ReturnValue` (`AbilitySystemComponent.GetGameplayAttributeValue` _abilitysystemcomponent (struct :`AttributeName` "Health" :`Attribute` "/Script/OneWeekProject_One.GGHealthSet:Health" :`AttributeOwner` "/Script/CoreUObject.Class'/Script/OneWeekProject_One.GGHealthSet'"))) (`.ReturnValue` (`AbilitySystemComponent.GetGameplayAttributeValue` _abilitysystemcomponent (struct :`AttributeName` "MaxHealth" :`Attribute` "/Script/OneWeekProject_One.GGHealthSet:MaxHealth" :`AttributeOwner` "/Script/CoreUObject.Class'/Script/OneWeekProject_One.GGHealthSet'")))))

(fn `UpdateShield`
  (bind _abilitysystemcomponent (`self.AbilitySystemComponent`))
  (bind _aswbp_health_bar (cast `/Game/UI/WBP_HealthBar` (`WidgetComponent.GetUserWidgetObject` (`self.HealthBar`))))
  (`/Game/UI/WBP_HealthBar.UpdateShield` _aswbp_health_bar (`.ReturnValue` (`AbilitySystemComponent.GetGameplayAttributeValue` _abilitysystemcomponent (struct :`AttributeName` "Shield" :`Attribute` "/Script/OneWeekProject_One.GGHealthSet:Shield" :`AttributeOwner` "/Script/CoreUObject.Class'/Script/OneWeekProject_One.GGHealthSet'"))) (`.ReturnValue` (`AbilitySystemComponent.GetGameplayAttributeValue` _abilitysystemcomponent (struct :`AttributeName` "MaxShield" :`Attribute` "/Script/OneWeekProject_One.GGHealthSet:MaxShield" :`AttributeOwner` "/Script/CoreUObject.Class'/Script/OneWeekProject_One.GGHealthSet'")))))

(fn `UserConstructionScript`)