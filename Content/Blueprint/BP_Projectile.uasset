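; BP_Projectile is a projectile actor that deals damage through the Gameplay Ability System when it hits something.
; On hit it prints the other actor's name, then checks that its owner and that actor both have ability system components.
; If so, it sets a fixed set-by-caller damage magnitude on the stored SpeedHandle effect spec and applies it from owner to target.
; It destroys itself after any hit.
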(event `self.ReceiveHit`
  (params (MyComp :type "PrimitiveComponent Object Reference") (Other :type "Actor Object Reference") (OtherComp :type "PrimitiveComponent Object Reference") (bSelfMoved :type Boolean) (HitLocation :type "Vector Structure") (HitNormal :type "Vector Structure") (NormalImpulse :type "Vector Structure") (Hit :type "HitResult Structure (by ref)"))
  (bind _returnvalue (`AbilitySystemBlueprintLibrary.GetAbilitySystemComponent` Other))
  (bind _returnvalue_2 (`AbilitySystemBlueprintLibrary.GetAbilitySystemComponent` (`self.GetOwner`)))
  (`KismetSystemLibrary.PrintString` (`KismetSystemLibrary.GetDisplayName` Other))
  (`|ExecutionSequence`
    (:`then_0`
      ; Check are they valid
      (`/Engine/EditorBlueprintResources/StandardMacros.IsValid` _returnvalue_2
        (:`Is Valid`
          (`/Engine/EditorBlueprintResources/StandardMacros.IsValid` _returnvalue
            (:`Is Valid`
              (bind _returnvalue_3 (`AbilitySystemBlueprintLibrary.AssignTagSetByCallerMagnitude` (`self.SpeedHandle`) (struct :`TagName` "Damage.SetByCaller") 10.0))
              (`AbilitySystemComponent.BP_ApplyGameplayEffectSpecToTarget` _returnvalue_2 _returnvalue_3 _returnvalue))))))
    (:`then_1`
      (`self.K2_DestroyActor`))))

(fn `UserConstructionScript`)