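; GA_FireAbility is a Gameplay Ability that fires a projectile along the character's camera aim.
; After committing, it spawns BP_Projectile ahead of the camera, offset by the spring arm length, passing it a GE_Damage effect spec from the character's ability system.
; The ability ends right after spawning or when the commit fails.
; An unconnected line-trace test that applies SetByCaller damage remains in the graph but never runs.
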(event `self.K2_ActivateAbility`
  (bind _character (`self.Character`))
  (bind _returnvalue (`AbilitySystemBlueprintLibrary.GetAbilitySystemComponent` (`self.Character`)))
  (bind _cameracomp (`GGPlayerCharacter.CameraComp` _character))
  (bind _returnvalue_2 (`SceneComponent.K2_GetComponentRotation` _cameracomp))
  (bind _asbp_character (cast `/Game/Characters/BP_Character` (`self.GetAvatarActorFromActorInfo`)))
  (set `self.Character` _asbp_character)
  (bind _returnvalue_3 (`self.K2_CommitAbility`))
  (if _returnvalue_3
    (`|ExecutionSequence`
      (:`then_0`
        (`|SpawnActorFromClass` "/Game/Blueprint/BP_Projectile.BP_Projectile_C" (`KismetMathLibrary.MakeTransform` (+ (`SceneComponent.K2_GetComponentLocation` _cameracomp) (* (`KismetMathLibrary.GetForwardVector` _returnvalue_2) (`SpringArmComponent.TargetArmLength` (`GGPlayerCharacter.SpringArmComp` _character)))) _returnvalue_2 (0.5 0.5 0.5)) "Undefined" "MultiplyWithRoot" (`self.Character`) (`AbilitySystemComponent.MakeOutgoingSpec` _returnvalue "/Game/GAS/Effects/GE_Damage.GE_Damage_C" 0.0 (`AbilitySystemComponent.MakeEffectContext` _returnvalue)) null))
      (:`then_1`
        ; End Ability
        (`self.K2_EndAbility` :!label _label)))
    (else
      (goto _label))))